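; BP_AIManager controls the single BP_AI enemy, detecting, chasing and catching the third-person player.
; It finds both actors at BeginPlay, then line-traces between them every Tick, starting a chase when the player is hit and stopping otherwise.
; An AI capsule overlap with the player fires the OnPlayerCatch dispatcher.
; It also forwards room-move requests to the AI and exposes its position.
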(event Custom|Event%20MoveToRoom
  (params (RoomPos :type Vector%20%28by%20ref%29))
  ;[1 1 1] Перемещение в заданную комнату
  (Default|EventMovetoRoom (Variables|Default|GetAI) RoomPos))

(event Custom|Event%20PlayerCatched
  (params (OverlappedComponent :type Primitive%20Component%20Object%20Reference) (OtherActor :type Actor%20Object%20Reference) (OtherComp :type Primitive%20Component%20Object%20Reference) (OtherBodyIndex :type Integer) (bFromSweep :type Boolean) (SweepResult :type Hit%20Result%20Structure%20%28by%20ref%29))
  ;[1 1 1] AI догнал игрока
  (Utilities|Casting|CastToBP_ThirdPersonCharacter OtherActor)
  (Default|CallOnPlayerCatch))

(event EventBeginPlay
  (bind _returnvalue (Actor|GetActorOfClass "/Game/Blueprints/AI/BP_AI.BP_AI_C"))
  (bind _output_get (Variables|Default|SetAI _returnvalue))
  (Collision|AssignOnComponentBeginOverlap (Variables|/Script/Engine.Character|GetCapsuleComponent _output_get) (EventDispatchers|CreateEvent :!event Custom|Event%20PlayerCatched))
  (bind _returnvalue_2 (Actor|GetActorOfClass "/Game/Blueprints/Player/BP_ThirdPersonCharacter.BP_ThirdPersonCharacter_C"))
  (Variables|Default|SetPlayer _returnvalue_2))

(event EventTick
  (params (DeltaSeconds :type Float%20%28single-precision%29))
  (bind _ai (Variables|Default|GetAI))
  (bind _ai_2 (Variables|Default|GetAI))
  (bind _ischasestarted (Variables|/Game/Blueprints/AI/BP_AI.BP_AI_C|GetIsChaseStarted _ai))
  ;[1 1 1] Ищет игрока, если тот оказывается в поле зрения, начинает его преследовать
  (bind _outhit (Collision|LineTraceForObjects (Transformation|GetActorLocation _ai_2) (Transformation|GetActorLocation (Variables|Default|GetPlayer)) (Utilities|Array|MakeArray "ObjectTypeQuery3" "ObjectTypeQuery1" "ObjectTypeQuery2") false (Utilities|Array|MakeArray _ai_2) "None"))
  (bind _asbp_third_person_character (Utilities|Casting|CastToBP_ThirdPersonCharacter (.HitActor (Collision|BreakHitResult _outhit)))
    (:then
      (if (not _ischasestarted)
        (Default|EventStartChase _ai _asbp_third_person_character)))
    (:CastFailed
      (if _ischasestarted
        (Default|EventStopChase _ai)))))

(fn ConstructionScript)

(fn GetAIPosition
  (return (Transformation|GetActorLocation (Variables|Default|GetAI))))