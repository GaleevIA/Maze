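; Manager that tracks rooms and doors and controls which doors are open around the player.
; On BeginPlay it caches all BP_Room and BP_Door actors, and it picks CurrentRoom using a 500-unit sphere overlap, nearest-distance check and line trace.
; Door requests and switches first close the current room's open doors, sparing one door type, then open the requested or a random eligible door.
; A separate event opens all entrance doors.
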(event Custom|Event%20OpenDoor
  (params (Door :type BP%20Door%20Object%20Reference%20%28by%20ref%29))
  ;[1 1 1] Открытие двери при запросе игрока
  (CallFunction|CloseDoors)
  (Default|EventOpen Door))

(event Custom|Event%20OpenEnterDoors
  ;[1 1 1] Открывает входные двери
  (for _array_element (Variables|Default|GetDoors)
    (if (Utilities|Enum|Equal(Enum) (Variables|/Game/Blueprints/BP_Door.BP_Door_C|GetType _array_element) "NewEnumerator0")
      (Default|EventOpen _array_element))))

(event Custom|Event%20SwitchDoors
  ;[1 1 1] Закрывает открытые двери и открывает случайную
  (CallFunction|CloseDoors)
  (bind _door (CallFunction|GetRandomDoor (Variables|Default|GetCurrentRoom)))
  (Utilities|IsValid _door
    (:Is%20Valid
      (Default|EventOpen _door))))

(event Custom|Event%20IdentifyCurrentRoom
  (params (CurPos :type Vector%20%28by%20ref%29))
  (bind _array (Utilities|Array|MakeArray "ObjectTypeQuery1" "ObjectTypeQuery2"))
  ;[1 1 1] Определяет текущую комнату игрока
  (bind _outactors (Collision|SphereOverlapActors CurPos 5e+02 _array "/Game/Blueprints/BP_Room.BP_Room_C"))
  (for _array_element _outactors
    (bind _outhit (Collision|LineTraceForObjects CurPos (Transformation|GetActorLocation _array_element) _array false 0 "ForDuration"))
    (if (< (Math|Vector|Distance(Vector) (Transformation|GetActorLocation _array_element) CurPos) (Variables|Default|GetDistanceToNearRoom))
      (Variables|Default|SetDistanceToNearRoom (Math|Vector|Distance(Vector) (Transformation|GetActorLocation _array_element) CurPos))
      (bind _asbp_room (Utilities|Casting|CastToBP_Room (.HitActor (Collision|BreakHitResult _outhit))))
      (Variables|Default|SetCurrentRoom _asbp_room)))
  (Variables|Default|SetDistanceToNearRoom 5e+02))

(event EventBeginPlay
  (bind _outactors (Actor|GetAllActorsOfClass "/Game/Blueprints/BP_Room.BP_Room_C"))
  (Variables|Default|SetRooms _outactors)
  (bind _outactors_2 (Actor|GetAllActorsOfClass "/Game/Blueprints/BP_Door.BP_Door_C"))
  (Variables|Default|SetDoors _outactors_2))

(fn ConstructionScript)

(fn CanbeOpened
  (params (Door :type BP%20Door%20Object%20Reference%20%28by%20ref%29))
  (return (and (not (Variables|/Game/Blueprints/BP_Door.BP_Door_C|GetIsOpened Door)) (Utilities|Enum|NotEqual(Enum) (Variables|/Game/Blueprints/BP_Door.BP_Door_C|GetType Door) "NewEnumerator0"))))

(fn GetRandomDoor
  (params (Room :type BP%20Room%20Object%20Reference%20%28by%20ref%29))
  (bind _temparray (LocalVariables|GetTempArray))
  (Utilities|IsValid Room
    (:Is%20Valid
      (for _array_element (Variables|/Game/Blueprints/BP_Room.BP_Room_C|GetDoors Room)
        (if (and (Utilities|Enum|Equal(Enum) (Variables|/Game/Blueprints/BP_Door.BP_Door_C|GetType _array_element) "NewEnumerator2") (not (Variables|/Game/Blueprints/BP_Door.BP_Door_C|GetIsOpened _array_element)))
          (Utilities|Array|Add (LocalVariables|GetTempArray) _array_element)))
      (return (Utilities|Array|Get(acopy) _temparray (Math|Random|RandomInteger (Utilities|Array|Length _temparray)))))))

(fn CloseDoors
  (bind _currentroom (Variables|Default|GetCurrentRoom))
  (Utilities|IsValid _currentroom
    (:Is%20Valid
      (for _array_element (Variables|/Game/Blueprints/BP_Room.BP_Room_C|GetDoors _currentroom)
        (if (and (Variables|/Game/Blueprints/BP_Door.BP_Door_C|GetIsOpened _array_element) (Utilities|Enum|NotEqual(Enum) (Variables|/Game/Blueprints/BP_Door.BP_Door_C|GetType _array_element) "NewEnumerator1"))
          (Default|EventClose _array_element))))))