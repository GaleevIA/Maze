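; BP_GameRulesManager decides when the game starts, stops and ends, based on checkpoint overlaps.
; On BeginPlay it binds to every BP_CheckPoint, then switches on PointType (Start, Finish, Stop), using state flags to filter repeats and broadcasting matching dispatchers.
; Start also runs a one-shot door-opening countdown, broadcasting timer start and end, with expiry, Finish and Stop all routed through StopTimer.
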(event Custom|Event%20OnCheckPointBeginOverlap
  (params (OverlappedActor :type Actor%20Object%20Reference) (OtherActor :type Actor%20Object%20Reference))
  ;[1 1 1] Определяет начало и окончание игры
  (bind _asbp_check_point (Utilities|Casting|CastToBP_CheckPoint OverlappedActor))
  (switch Utilities|FlowControl|Switch|SwitchonE_CheckPointType (Variables|/Game/Blueprints/BP_CheckPoint.BP_CheckPoint_C|GetPointType _asbp_check_point)
    (:NewEnumerator0
      (if (not (Variables|Default|GetIsGameStarted))
        (Variables|Default|SetIsGameStarted true)
        (Default|CallOnGameStart)
        (CallFunction|EventStartTimer)))
    (:NewEnumerator1
      (if (not (Variables|Default|GetIsGameEnded))
        (Variables|Default|SetIsGameEnded true)
        (Default|CallOnGameEnd true)
        (CallFunction|EventStopTimer)))
    (:NewEnumerator2
      (if (Variables|Default|GetIsGameStarted)
        (Variables|Default|SetIsGameStarted false)
        (Default|CallOnGameStop)
        (CallFunction|EventStopTimer)))))

(event Custom|Event%20StartTimer
  ;[1 1 1] Включает и отключает таймер до открытия новой двери
  (bind _returnvalue (Utilities|Time|SetTimerbyEvent (delegate Custom|Event%20StopTimer) 1e+01))
  (Default|CallOnTimerStart))

(event Custom|Event%20StopTimer
  ;[1 1 1] Включает и отключает таймер до открытия новой двери
  (Utilities|Time|ClearandInvalidateTimerbyHandle (stale Custom|Event%20StartTimer _returnvalue))
  (Default|CallOnTimerEnd))

(event EventBeginPlay
  (bind _outactors (Actor|GetAllActorsOfClass "/Game/Blueprints/BP_CheckPoint.BP_CheckPoint_C"))
  (bind _output_get (Variables|Default|SetCheckPoints _outactors))
  (for _array_element _output_get
    (EventDispatchers|AssignOnActorBeginOverlap _array_element (EventDispatchers|CreateEvent :!event Custom|Event%20OnCheckPointBeginOverlap))))

(fn ConstructionScript)