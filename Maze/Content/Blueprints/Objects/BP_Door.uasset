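; BP_Door is a door actor that opens and closes by rotating its mesh, with two point lights reflecting its state.
; Open and Close events play the OpenCloseDoor timeline forward from the start or backward from the end, driving the mesh's relative yaw.
; When the timeline finishes, it toggles IsOpened and calls SwitchLight, which makes both lights bright when open and dim when closed.
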(event Custom|Event%20Open
  ;[1 1 1] Открытие/закрытие двери
  (bind _z_rotation (Timeline|OpenCloseDoor PlayFromStart)
    (:Update
      (Transformation|SetRelativeRotation (Variables|Default|GetSM_Door) (Math|Rotator|MakeRotator 0.0 0.0 _z_rotation) false false))
    (:Finished
      (Variables|Default|SetIsOpened (not (Variables|Default|GetIsOpened)))
      (CallFunction|SwitchLight))))

(event Custom|Event%20Close
  ;[1 1 1] Открытие/закрытие двери
  (bind _z_rotation (Timeline|OpenCloseDoor ReverseFromEnd)
    (:Update
      (Transformation|SetRelativeRotation (Variables|Default|GetSM_Door) (Math|Rotator|MakeRotator 0.0 0.0 _z_rotation) false false))
    (:Finished
      (Variables|Default|SetIsOpened (not (Variables|Default|GetIsOpened)))
      (CallFunction|SwitchLight))))

(fn ConstructionScript)

(fn SwitchLight
  (if (Variables|Default|GetIsOpened)
    (LocalVariables|SetNewIntensity 1e+04)
    (else
      (LocalVariables|SetNewIntensity 1e+02)))
  (Rendering|Components|Light|SetIntensity (Variables|Default|GetPointLight1) (LocalVariables|GetNewIntensity))
  (Rendering|Components|Light|SetIntensity (Variables|Default|GetPointLight) (LocalVariables|GetNewIntensity)))