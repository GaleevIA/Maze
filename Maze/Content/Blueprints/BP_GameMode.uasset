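; Game mode for a room-and-door chase game where the player loses if the AI catches them.
; BeginPlay spawns AI, rooms and game rules managers, then binds their events, plus character and HUD events, acting as central mediator.
; Player door interaction or timer expiry makes the rooms manager open or switch doors, sends the AI to its next room, and restarts the countdown after a delay.
; HUD shows prompts, timer and game-over, and restarts the level.
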(event Custom|HUD_OnRestart
  ;[1 1 1] Перезапуск уровня
  (bind _returnvalue (Game|GetCurrentLevelName true))
  (Game|OpenLevel(byName) (Utilities|String|StringToName _returnvalue)))

(event Custom|Player_OnDoorHighlighted
  (params (IsHighlighted :type Boolean) (Door :type BP%20Door%20Object%20Reference))
  ;[1 1 1] Вывод панели взаимодействия при приближении к двери игроком
  (if IsHighlighted
    (bind _can (Default|CanbeOpened (Variables|Default|GetManagerRooms) Door))
    (if _can
      (Default|EventShowInteractWidget (Variables|Default|GetHUD)))
    (else
      (Default|EventHideInteractWidget (Variables|Default|GetHUD)))))

(event Custom|Player_OnDoorInteract
  (params (Door :type BP%20Door%20Object%20Reference))
  (bind _managerrooms (Variables|Default|GetManagerRooms))
  ;[1 1 1] Взаимодействие игрока с дверью
  (bind _can (Default|CanbeOpened _managerrooms Door))
  (if _can
    (bind _position (Default|GetAIPosition (Variables|Default|GetManagerAI)))
    (Default|EventOpenDoor _managerrooms Door (Transformation|GetActorLocation (Game|Player|GetPlayerPawn 0)) _position)
    (Default|EventMovetoRoom (Variables|Default|GetManagerAI) (Transformation|GetActorLocation (Variables|/Game/Blueprints/Managers/BP_RoomsManager.BP_RoomsManager_C|GetNextAIRoom (Variables|Default|GetManagerRooms))))
    (Default|EventHideTimerWidget (Variables|Default|GetHUD))
    (Utilities|FlowControl|Delay 2.0)
    (Default|EventStartTimer (Variables|Default|GetManagerGameRules))))

(event Custom|Game_OnTimerEnd
  ;[1 1 1] Окончания таймера открытия двери
  (Default|EventHideTimerWidget (Variables|Default|GetHUD))
  (if (and (Variables|Default|GetIsGameStarted) (not (Variables|Default|GetIsGameFinished)))
    (bind _position (Default|GetAIPosition (Variables|Default|GetManagerAI)))
    (Default|EventSwitchDoors (Variables|Default|GetManagerRooms) (Transformation|GetActorLocation (Game|Player|GetPlayerPawn 0)) _position)
    (Default|EventMovetoRoom (Variables|Default|GetManagerAI) (Transformation|GetActorLocation (Variables|/Game/Blueprints/Managers/BP_RoomsManager.BP_RoomsManager_C|GetNextAIRoom (Variables|Default|GetManagerRooms))))
    (Utilities|FlowControl|Delay 2.0)
    (Default|EventStartTimer (Variables|Default|GetManagerGameRules))))

(event Custom|Game_OnStart
  ;[1 1 1] Начало игры
  (Variables|Default|SetIsGameStarted true))

(event Custom|Game_OnStop
  ;[1 1 1] Остановка игры, если игрок вышел из зеленой двери
  (Variables|Default|SetIsGameStarted false)
  (Default|EventHideTimerWidget (Variables|Default|GetHUD)))

(event Custom|Game_OnEnd
  (params (IsWin :type Boolean))
  ;[1 1 1] Окончания игры
  (Variables|Default|SetIsGameFinished true)
  (Default|EventShowGameOverWidget (Variables|Default|GetHUD) IsWin))

(event Custom|AI_OnPlayerCatch
  ;[1 1 1] Игрок был пойман
  (CallFunction|GameonEnd false))

(event Custom|Game_OnTimerStart
  ;[1 1 1] Включение таймера до открытия двери
  (Default|EventShowTimerWidget (Variables|Default|GetHUD)))

(event EventBeginPlay
  ;[1 1 1] Создает менеджеры и подписывается на события
  (CallFunction|InitializeAIManager)
  (CallFunction|InitializeRoomsManager)
  (CallFunction|InitializeGameRulesManager)
  (CallFunction|InitializePlayer)
  (CallFunction|InitializeHUD)
  (Default|EventOpenEnterDoors (Variables|Default|GetManagerRooms)))

(fn ConstructionScript)

(fn InitializeAIManager
  (bind _returnvalue (Game|SpawnActorfromClass "/Game/Blueprints/Managers/BP_AIManager.BP_AIManager_C" (Math|Transform|MakeTransform "0, 0, 0" "0, 0, 0" "1,1,1") "Undefined" 0 0))
  (bind _output_get (Variables|Default|SetManagerAI _returnvalue))
  (EventDispatchers|BindEventtoOnPlayerCatch _output_get (EventDispatchers|CreateEvent :!event Custom|AI_OnPlayerCatch)))

(fn InitializeRoomsManager
  (bind _returnvalue (Game|SpawnActorfromClass "/Game/Blueprints/Managers/BP_RoomsManager.BP_RoomsManager_C" (Math|Transform|MakeTransform "0, 0, 0" "0, 0, 0" "1,1,1") "Undefined" 0 0))
  (Variables|Default|SetManagerRooms _returnvalue))

(fn InitializeGameRulesManager
  (bind _returnvalue (Game|SpawnActorfromClass "/Game/Blueprints/Managers/BP_GameRulesManager.BP_GameRulesManager_C" (Math|Transform|MakeTransform "0, 0, 0" "0, 0, 0" "1,1,1") "Undefined" 0 0))
  (bind _output_get (Variables|Default|SetManagerGameRules _returnvalue))
  (EventDispatchers|BindEventtoOnTimerStart _output_get (EventDispatchers|CreateEvent :!event Custom|Game_OnTimerStart))
  (EventDispatchers|BindEventtoOnTimerEnd _output_get (EventDispatchers|CreateEvent :!event Custom|Game_OnTimerEnd))
  (EventDispatchers|BindEventtoOnGameStart _output_get (EventDispatchers|CreateEvent :!event Custom|Game_OnStart))
  (EventDispatchers|BindEventtoOnGameEnd _output_get (EventDispatchers|CreateEvent :!event Custom|Game_OnEnd))
  (EventDispatchers|BindEventtoOnGameStop _output_get (EventDispatchers|CreateEvent :!event Custom|Game_OnStop)))

(fn InitializePlayer
  (bind _asbp_third_person_character (Utilities|Casting|CastToBP_ThirdPersonCharacter (Game|Player|GetPlayerPawn 0)))
  (EventDispatchers|BindEventtoOnDoorHighlighted _asbp_third_person_character (EventDispatchers|CreateEvent :!event Custom|Player_OnDoorHighlighted))
  (EventDispatchers|BindEventtoOnDoorInteract _asbp_third_person_character (EventDispatchers|CreateEvent :!event Custom|Player_OnDoorInteract)))

(fn InitializeHUD
  (bind _asbp_hud (Utilities|Casting|CastToBP_HUD (HUD|GetHUD (Game|GetPlayerController 0))))
  (bind _output_get (Variables|Default|SetHUD _asbp_hud))
  (EventDispatchers|BindEventtoOnRestartClicked _output_get (EventDispatchers|CreateEvent :!event Custom|HUD_OnRestart)))