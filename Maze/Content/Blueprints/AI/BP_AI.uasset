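; BP_AI is an AI-controlled pawn that moves to room positions and can chase a player.
; MoveToRoom stores the given position as LastPosition and issues AIMoveTo toward it.
; StartChase sets IsChaseStarted and moves toward the player actor, while StopChase clears the flag and sends the pawn back to LastPosition.
; All three behaviors are events with no decision logic of their own.
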(event Custom|Event%20MoveToRoom
  (params (RoomPos :type Vector))
  ;[1 1 1] Идет в комнату
  (bind _output_get (Variables|Default|SetLastPosition RoomPos))
  (AI|AIMoveTo self _output_get 0 5.0 false))

(event Custom|Event%20StartChase
  (params (Player :type Actor%20Object%20Reference))
  ;[1 1 1] Начинает погоню за игроком
  (Variables|Default|SetIsChaseStarted true)
  (AI|AIMoveTo self "0, 0, 0" Player 5.0 false))

(event Custom|Event%20StopChase
  ;[1 1 1] Заканчивает погоню за игроком
  (Variables|Default|SetIsChaseStarted false)
  (AI|AIMoveTo self (Variables|Default|GetLastPosition) 0 5.0 false))

(fn ConstructionScript)